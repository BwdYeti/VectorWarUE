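; Spawner actor that creates the visible ship and bullet actors for a Vector War match on BeginPlay.
; It reads the ship and bullet counts from VWGameStateBase and spawns that many BP_VectorWarShip and BP_VectorWarBullet actors at its root transform.
; Each spawned actor receives its player or bullet index and is stored in the Ships or Bullets array.
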(event `self.ReceiveBeginPlay`
  (`self.SpawnShips`)
  (`self.SpawnBullets`))

(fn `SpawnBullets`
  (bind _asvwgame_state_base (cast `VWGameStateBase` (`GameplayStatics.GetGameState`)))
  (for _index (range (`GameStateInterface.BulletCount` _asvwgame_state_base))
    (`|SpawnActorFromClass` "/Game/Blueprints/BP_VectorWarBullet.BP_VectorWarBullet_C" (`SceneComponent.K2_GetComponentToWorld` (`self.Root`)) "Undefined" "OverrideRootScale" null _index null)
    (`KismetArrayLibrary.Array_Add` (`self.Bullets`))))

(fn `SpawnShips`
  (bind _asvwgame_state_base (cast `VWGameStateBase` (`GameplayStatics.GetGameState`)))
  (for _index (range (`GameStateInterface.ShipCount` _asvwgame_state_base))
    (bind _returnvalue (`|SpawnActorFromClass` "/Game/Blueprints/BP_VectorWarShip.BP_VectorWarShip_C" (`SceneComponent.K2_GetComponentToWorld` (`self.Root`)) "Undefined" "OverrideRootScale" null _index null))
    (`KismetArrayLibrary.Array_Add` (`self.Ships`) _returnvalue)))

(fn `UserConstructionScript`)